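; Player-controllable tank Blueprint that maps input to track driving, camera aiming and firing.
; BeginPlay passes the barrel and turret components to native-style setters, while the construction script assigns turret and track meshes.
; Track throttle axes drive each track directly, and MoveForward goes through TankMovementComponent; MoveBackward is empty.
; Aim axes rotate the azimuth gimbal in yaw and spring arm in pitch separately, and Fire calls Fire().
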(event `self.ReceiveBeginPlay`
  (`self.SetBarrelReference` (`self.TankBarrel1`))
  (`self.SetTurretReference` (`self.TankTurret`)))

(event `InputAxis|LeftTrackThrottle`
  (params (AxisValue :type "Float (single-precision)"))
  ;[1 1 1] Movment Input
  (`TankTracks.SetThrottle` (`self.Left Track`) AxisValue))

(event `InputAxis|AimAzimuth`
  (params (AxisValue :type "Float (single-precision)"))
  ;[1 1 1] Aiming Input
  (`SceneComponent.K2_AddLocalRotation` (`self.Azimuth Gimbal`) (`KismetMathLibrary.MakeRotator` 0.0 0.0 AxisValue) false false))

(event `InputAxis|RightTrackThrottle`
  (params (AxisValue :type "Float (single-precision)"))
  ;[1 1 1] Movment Input
  (`TankTracks.SetThrottle` (`self.Right Track`) AxisValue))

(event `InputAxis|AimAltitude`
  (params (AxisValue :type "Float (single-precision)"))
  ;[1 1 1] Aiming Input
  (`SceneComponent.K2_AddLocalRotation` (`self.SpringArm`) (`KismetMathLibrary.MakeRotator` 0.0 AxisValue) false false))

(event `InputAxis|MoveForward`
  (params (AxisValue :type "Float (single-precision)"))
  ;[1 1 1] Movment Input
  (`TankMovementComponent.IntendMoveForward` (`self.TankMovementComponent`) AxisValue))

(event `InputAction|Fire`
  (params (Key :type "Key Structure"))
  ;[1 1 1] Aiming Input
  (:`Pressed`
    (`self.Fire`)))

(event `InputAxis|MoveBackward`
  (params (AxisValue :type "Float (single-precision)"))
  ;[1 1 1] Movment Input
)

(fn `UserConstructionScript`
  (`StaticMeshComponent.SetStaticMesh` (`self.TankTurret`) "/Game/Tank/tank_fbx_Turret.tank_fbx_Turret")
  (`StaticMeshComponent.SetStaticMesh` (`self.Left Track`) "/Game/Tank/tank_fbx_Track.tank_fbx_Track")
  (`StaticMeshComponent.SetStaticMesh` (`self.Right Track`) "/Game/Tank/tank_fbx_Track.tank_fbx_Track"))